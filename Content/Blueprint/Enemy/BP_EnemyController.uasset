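; BP_EnemyController is the AI controller for enemies, setting up blackboard data and starting their behavior tree.
; On BeginPlay it initializes BB_Enemy, seeding the target location with the controlled pawn's position and the home location with a random navigable point nearby.
; It then runs BT_Enemy and holds no per-frame logic of its own.
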(event EventBeginPlay
  (bind _returnvalue (Pawn|GetControlledPawn))
  (bind _returnvalue_2 (Transformation|GetActorLocation _returnvalue))
  (Utilities|FlowControl|Sequence
    (:then_0
      (Class|AIController|UseBlackboard "/Game/Blueprint/Enemy/AI/BB_Enemy.BB_Enemy")
      (AI|Components|Blackboard|SetValueasVector (Variables|Default|GetBlackboard) (Variables|Default|GetTargetLocationKey) _returnvalue_2)
      (AI|Components|Blackboard|SetValueasVector (Variables|Default|GetBlackboard) (Variables|Default|GetHomeLocationKey) (.RandomLocation (Class|NavigationSystem|GetRandomPointinNavigableRadius _returnvalue_2 6e+02))))
    (:then_1
      (AI|RunBehaviorTree "/Game/Blueprint/Enemy/AI/BT_Enemy.BT_Enemy"))))

(event EventTick
  (params (DeltaSeconds :type Float%20%28single-precision%29)))

(fn ConstructionScript)