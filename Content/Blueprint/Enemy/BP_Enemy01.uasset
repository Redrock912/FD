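; BP_Enemy01 is an enemy that tracks HP and a state enum, and drops gold when killed.
; AnyDamage accepts only BP_CPP_Operator causers, storing their DeathImpactVector and subtracting HP until OnDead fires.
; OnDead disables capsule collision, spawns BP_DroppedItemGold above the body, ragdolls the mesh with a force along the stored vector, and sets a short lifespan.
; SetState lets callers change state except out of the dead state.
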(event Custom|OnDead
  (Variables|Default|SetState "NewEnumerator3")
  (Collision|SetCollisionEnabled (Variables|Collision|GetCapsuleComponent) "NoCollision")
  (Game|SpawnActorfromClass "/Game/Blueprint/Item/BP_DroppedItemGold.BP_DroppedItemGold_C" (Math|Transform|MakeTransform (+ (Transformation|GetActorLocation) "0, 0,200.000000") "0, 0, 0" "1,1,1") "Undefined" 0 0)
  (Actor|SetLifeSpan 5.0)
  (Physics|SetSimulatePhysics (Variables|Character|GetMesh) true)
  (Physics|AddForce (Variables|Character|GetMesh) (* (Math|Vector|Normalize (Variables|Default|GetImpactForce)) 2e+06) "None" false))

(event Custom|SetState
  (params (NewParam :type E_EnemyState%20Enum :default "NewEnumerator0"))
  (if (Utilities|Enum|NotEqual(Enum) (Variables|Default|GetState) "NewEnumerator3")
    (Variables|Default|SetState NewParam)))

(event EventBeginPlay
  (Variables|Default|SetState "NewEnumerator0"))

(event Collision|EventActorBeginOverlap
  (params (OtherActor :type Actor%20Object%20Reference)))

(event EventTick
  (params (DeltaSeconds :type Float%20%28single-precision%29)))

(event Game|Damage|EventAnyDamage
  (params (Damage :type Float%20%28single-precision%29) (DamageType :type Damage%20Type%20Object%20Reference) (InstigatedBy :type Controller%20Object%20Reference) (DamageCauser :type Actor%20Object%20Reference))
  (bind _asbp_cpp_operator (Utilities|Casting|CastToBP_CPP_Operator DamageCauser))
  (Variables|Default|SetImpactForce (Variables|/Script/topView.Operator|GetDeathImpactVector _asbp_cpp_operator))
  (Variables|Default|SetCurrentHP (- (Variables|Default|GetCurrentHP) Damage))
  (if (not (> (Variables|Default|GetCurrentHP) 0.0))
    (CallFunction|OnDead)))

(fn ConstructionScript)