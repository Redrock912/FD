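; BP_DroppedItem is a dropped item actor that gets a random physics push when it spawns.
; On BeginPlay it stores a random unit vector and applies a one-time AddForce along it to the static mesh, scaled randomly between minimum and maximum impact force variables.
; The construction script lowers the mesh's mass scale, and there is no overlap or tick logic.
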(event EventBeginPlay
  (Variables|Default|SetImpactVector (Math|Random|RandomUnitVector))
  (Physics|AddForce (Variables|Debug|GetStaticMeshComponent) (* (Variables|Default|GetImpactVector) (Math|Random|RandomFloatinRange (Variables|Default|GetImpactForceMin) (Variables|Default|GetImpactFoceMax))) "None" false))

(event Collision|EventActorBeginOverlap
  (params (OtherActor :type Actor%20Object%20Reference)))

(event EventTick
  (params (DeltaSeconds :type Float%20%28single-precision%29)))

(fn ConstructionScript
  (Class|PrimitiveComponent|SetMassScale (Variables|Debug|GetStaticMeshComponent) "None" 0.2))